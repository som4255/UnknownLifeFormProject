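; Player character Blueprint that commands a companion AI and interacts with world actors.
; It spawns a BP_FriendlyAI beside itself on BeginPlay, and Hold, Follow and Recon inputs set that companion's AIWork state.
; The interact input triggers the current TriggerAct's Interacted, while SetAIETC switches the companion's work state and passes that actor to its AI controller.
; Each tick, a spotlight's rotation follows the camera's forward vector.
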(event EventBeginPlay
  (bind _returnvalue (Transformation|GetActorTransform))
  (bind (_location _rotation) (Math|Transform|BreakTransform _returnvalue))
  (bind _returnvalue_2 (Game|SpawnActorfromClass "/Game/01_FriendlyAI/BP_FriendlyAI.BP_FriendlyAI_C" (Math|Transform|MakeTransform (+ _location (* (Transformation|GetActorRightVector) 2e+02) "0.000000,0.000000,-6.000000") _rotation) "AdjustIfPossibleButAlwaysSpawn" "MultiplyWithRoot" 0 0))
  (Utilities|IsValid _returnvalue_2
    (:Is%20Valid
      (Variables|Default|SetFriendlyAI _returnvalue_2))
    (:Is%20Not%20Valid
      (Development|PrintString "FriendlyAIFailCast"))))

(event EventTick
  (params (DeltaSeconds :type Float%20%28single-precision%29))
  (Transformation|SetWorldRotation (Variables|Default|GetSpotLight) (Math|Conversions|RotationFromXVector (Math|Vector|GetForwardVector (Variables|Default|Getm_Camera))) false false))

(event Input|ActionEvents|InputActionHold
  (params (Key :type Key%20Structure :default "None"))
  (bind _friendlyai (Variables|Default|GetFriendlyAI))
  (:Pressed
    (Utilities|IsValid _friendlyai
      (:Is%20Valid
        (Variables|/Game/01_FriendlyAI/BP_FriendlyAI.BP_FriendlyAI_C|SetAIWork _friendlyai "NewEnumerator0")))))

(event Input|ActionEvents|InputActionFollow
  (params (Key :type Key%20Structure :default "None"))
  (bind _friendlyai (Variables|Default|GetFriendlyAI))
  (:Pressed
    (Utilities|IsValid _friendlyai
      (:Is%20Valid
        (Variables|/Game/01_FriendlyAI/BP_FriendlyAI.BP_FriendlyAI_C|SetAIWork _friendlyai "NewEnumerator1")))))

(event Input|ActionEvents|InputActionRecon
  (params (Key :type Key%20Structure :default "None"))
  (bind _friendlyai (Variables|Default|GetFriendlyAI))
  (:Pressed
    (Utilities|IsValid _friendlyai
      (:Is%20Valid
        (Variables|/Game/01_FriendlyAI/BP_FriendlyAI.BP_FriendlyAI_C|SetAIWork _friendlyai "NewEnumerator2")))))

(event Input|ActionEvents|InputActionInteractedActor
  (params (Key :type Key%20Structure :default "None"))
  (bind _triggeract (Variables|Default|GetTriggerAct))
  (:Pressed
    (Utilities|IsValid _triggeract
      (:Is%20Valid
        (bind _asbp_interacted_actor (Utilities|Casting|CastToBP_InteractedActor _triggeract)
          (:then
            (Default|Interacted _asbp_interacted_actor))
          (:CastFailed
            (Development|PrintString "PlayerCharacter::InteractedActorCastFail" true true "(R=0.000000,G=0.660000,B=1.000000,A=1.000000)" 1e+01)))))))

(fn ConstructionScript)

(fn SetAIETC
  (bind _friendlyai (Variables|Default|GetFriendlyAI))
  (Variables|/Game/01_FriendlyAI/BP_FriendlyAI.BP_FriendlyAI_C|SetAIWork _friendlyai "NewEnumerator3")
  (bind _asctr_aicontroller (Utilities|Casting|CastToCTR_AIController (AI|GetAIController _friendlyai))
    (:then
      (bind _asbp_interacted_actor (Utilities|Casting|CastToBP_InteractedActor (Variables|Default|GetTriggerAct))
        (:then
          (Default|SetAIWorkEtc _asctr_aicontroller _asbp_interacted_actor))
        (:CastFailed
          (Development|PrintString "BP_Character::SetAIEtc::InteractedActorCastFail" true true "(R=0.000000,G=0.660000,B=1.000000,A=1.000000)" 1e+01))))
    (:CastFailed
      (Development|PrintString "BP_Character::SetAIEtc::AIConterollerCastFail"))))