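; Interactable generator prop for the hotel map that unlocks a linked switch and, when operated, starts spawning.
; Box overlap registers it as the player character's trigger actor and shows or hides the HUD interaction prompt.
; Interaction is single-use: it calls SetAIETC on the player, enables the Switch and collapses the prompt.
; Operate, a separate entry point, plays audio, runs parent logic and activates all SpawnTrigger spawn volumes.
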(event OnComponentBeginOverlap(Box)
  (params (OverlappedComponent :type Primitive%20Component%20Object%20Reference) (OtherActor :type Actor%20Object%20Reference) (OtherComp :type Primitive%20Component%20Object%20Reference) (OtherBodyIndex :type Integer) (bFromSweep :type Boolean) (SweepResult :type Hit%20Result%20Structure%20%28by%20ref%29))
  (bind _asbp_sac1character (Utilities|Casting|CastToBP_SAC1Character OtherActor)
    (:then
      (Variables|/Game/KBJ/BluePrints/BP_SAC1Character.BP_SAC1Character_C|SetTriggerAct _asbp_sac1character self)
      (Variables|Default|SetPlayer _asbp_sac1character)
      (if (Variables|Default|GetCanUse)
        (bind _assac1hud (Utilities|Casting|CastToSAC1HUD (HUD|GetHUD (Game|GetPlayerController 0)))
          (:then
            (Class|SAC1HUD|SetInteractionText _assac1hud "Visible" (Variables|Default|GetName)))
          (:CastFailed
            (Development|PrintString "Interactedactor::HUDCasatFail" true true "(R=0.000000,G=0.660000,B=1.000000,A=1.000000)" 1e+01)))))
    (:CastFailed
      (Development|PrintString "InteractedActerCharacterCastFail"))))

(event OnComponentEndOverlap(Box)
  (params (OverlappedComponent :type Primitive%20Component%20Object%20Reference) (OtherActor :type Actor%20Object%20Reference) (OtherComp :type Primitive%20Component%20Object%20Reference) (OtherBodyIndex :type Integer))
  (bind _asbp_sac1character (Utilities|Casting|CastToBP_SAC1Character OtherActor)
    (:then
      (Variables|/Game/KBJ/BluePrints/BP_SAC1Character.BP_SAC1Character_C|SetTriggerAct _asbp_sac1character 0)
      (if (Variables|Default|GetCanUse)
        (bind _assac1hud (Utilities|Casting|CastToSAC1HUD (HUD|GetHUD (Game|GetPlayerController 0)))
          (:then
            (Class|SAC1HUD|SetInteractionText _assac1hud "Collapsed" (Variables|Default|GetName)))
          (:CastFailed
            (Development|PrintString "Interactedactor::HUDCasatFail" true true "(R=0.000000,G=0.660000,B=1.000000,A=1.000000)" 1e+01)))))
    (:CastFailed
      (Development|PrintString "InteractedActerCharacterCastFail"))))

(event Custom|Interaction
  (bind _switch (Variables|Default|GetSwitch))
  (if (Variables|Default|GetCanUse)
    (Variables|Default|SetCanUse false)
    (Default|SetAIETC (Variables|Default|GetPlayer))
    (Utilities|IsValid _switch
      (:Is%20Valid
        (Variables|/Game/00_HotelMap/Prop/Blueprint/Switch/BP_Switch.BP_Switch_C|SetCanUseSwitch _switch true))
      (:Is%20Not%20Valid
        _))
    (bind _assac1hud (Utilities|Casting|CastToSAC1HUD (HUD|GetHUD (Game|GetPlayerController 0)))
      (:then
        (Class|SAC1HUD|SetInteractionText _assac1hud "Collapsed" (Variables|Default|GetName)))
      (:CastFailed
        (Development|PrintString "Interactedactor::HUDCasatFail" true true "(R=0.000000,G=0.660000,B=1.000000,A=1.000000)" 1e+01)))))

(fn ConstructionScript
  (|CallParentFunction))

(fn Interacted
  (CallFunction|Interaction))

(fn Operate
  (Audio|Components|Audio|Play (Variables|Default|GetAudio) 0.0)
  (|CallParentFunction)
  (for _array_element (Variables|/Script/SAC1.TriggerRamdomSpawn|Getm_SpawnVolumes (Variables|Default|GetSpawnTrigger))
    (Class|ActorSpawnVolume|SetSpawningActive _array_element true)))