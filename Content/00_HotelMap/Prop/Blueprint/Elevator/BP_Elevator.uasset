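; BP_Elevator is an interactable hotel elevator that takes the player to another level.
; Its box overlap registers it as the character's TriggerAct and toggles the HUD interaction prompt while it is usable.
; Interacting disables further use and calls SetAIETC on the player.
; The separate Operate override, not called within this graph, opens the level named by LevelName.
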(event OnComponentBeginOverlap(Box)
  (params (OverlappedComponent :type Primitive%20Component%20Object%20Reference) (OtherActor :type Actor%20Object%20Reference) (OtherComp :type Primitive%20Component%20Object%20Reference) (OtherBodyIndex :type Integer) (bFromSweep :type Boolean) (SweepResult :type Hit%20Result%20Structure%20%28by%20ref%29))
  (bind _asbp_sac1character (Utilities|Casting|CastToBP_SAC1Character OtherActor)
    (:then
      (Variables|/Game/KBJ/BluePrints/BP_SAC1Character.BP_SAC1Character_C|SetTriggerAct _asbp_sac1character self)
      (Variables|Default|SetPlayer _asbp_sac1character)
      (if (Variables|Default|GetCanUse)
        (bind _assac1hud (Utilities|Casting|CastToSAC1HUD (HUD|GetHUD (Game|GetPlayerController 0)))
          (:then
            (Class|SAC1HUD|SetInteractionText _assac1hud "Visible" (Variables|Default|GetName)))
          (:CastFailed
            (Development|PrintString "Interactedactor::HUDCasatFail" true true "(R=0.000000,G=0.660000,B=1.000000,A=1.000000)" 1e+01)))))
    (:CastFailed
      (Development|PrintString "InteractedActerCharacterCastFail"))))

(event OnComponentEndOverlap(Box)
  (params (OverlappedComponent :type Primitive%20Component%20Object%20Reference) (OtherActor :type Actor%20Object%20Reference) (OtherComp :type Primitive%20Component%20Object%20Reference) (OtherBodyIndex :type Integer))
  (bind _asbp_sac1character (Utilities|Casting|CastToBP_SAC1Character OtherActor)
    (:then
      (Variables|/Game/KBJ/BluePrints/BP_SAC1Character.BP_SAC1Character_C|SetTriggerAct _asbp_sac1character 0)
      (if (Variables|Default|GetCanUse)
        (bind _assac1hud (Utilities|Casting|CastToSAC1HUD (HUD|GetHUD (Game|GetPlayerController 0)))
          (:then
            (Class|SAC1HUD|SetInteractionText _assac1hud "Collapsed" (Variables|Default|GetName)))
          (:CastFailed
            (Development|PrintString "Interactedactor::HUDCasatFail" true true "(R=0.000000,G=0.660000,B=1.000000,A=1.000000)" 1e+01)))))
    (:CastFailed
      (Development|PrintString "InteractedActerCharacterCastFail"))))

(event Custom|Interaction
  (if (Variables|Default|GetCanUse)
    (Variables|Default|SetCanUse false)
    (Default|SetAIETC (Variables|Default|GetPlayer))))

(fn ConstructionScript
  (|CallParentFunction))

(fn Interacted
  (CallFunction|Interaction))

(fn Operate
  (|CallParentFunction)
  (Game|OpenLevel(byName) (Variables|Default|GetLevel%20Name)))